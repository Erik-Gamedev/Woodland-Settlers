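; BP_Worker is a worker unit that moves to a requested location on command.
; MovetoThisLocation casts its controller to BP_CameraController, passes it to SimpleMoveToLocation and logs a fixed success string without checking the result.
; Tab calls SetViewTargetWithBlend on the player controller with no target specified.
; An AIMoveTo alternative is disconnected, and CustomEvent and GoTotThisLocation are empty stubs.
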(event `Key|Tab`
  (params (Key :type "Key Structure"))
  (:`Pressed`
    (`PlayerController.SetViewTargetWithBlend` (`GameplayStatics.GetPlayerController` 0) null 0.0 "VTBlend_Linear" 0.0 false)))

(event `self.ReceiveBeginPlay`)

(event `/Game/Blueprints/Worker/BPI_WorkerActions.MoveToThisLocation`
  (params (GoLocation :type "Vector Structure"))
  (bind _asbp_camera_controller (cast `/Game/Blueprints/Camera/BP_CameraController` (`self.GetController`))
    (:`then`
      _)
    (:`CastFailed`
      (`KismetSystemLibrary.PrintString` "Cast failed")))
  (`AIBlueprintHelperLibrary.SimpleMoveToLocation` _asbp_camera_controller GoLocation)
  (`KismetSystemLibrary.LogString` "Succeeded"))

(event `CustomEvent`
  (params (GoLocation :type "Vector Structure")))

(fn `GoTotThisLocation`
  (params (`Goal Location` :type "Vector Structure")))

(fn `UserConstructionScript`)