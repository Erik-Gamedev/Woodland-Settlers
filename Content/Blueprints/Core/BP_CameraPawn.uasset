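; Player camera pawn that pans with Enhanced Input and shows the mouse cursor.
; BeginPlay adds the default mapping context and caches a reference to the pawn through CastReference.
; IA_MoveCamera feeds AddMovementInput along right and forward vectors derived from control rotation.
; An alternative transform-based movement, with speed scaled by spring arm length and clamped, is left disconnected and never runs.
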(event `self.ReceiveBeginPlay`
  (bind _asplayer_controller (cast `PlayerController` (`self.GetController`)))
  (bind _returnvalue (pcsubsystem `EnhancedInputLocalPlayerSubsystem` _asplayer_controller))
  (`/Engine/EditorBlueprintResources/StandardMacros.IsValid` _returnvalue
    (:`Is Valid`
      (`EnhancedInputSubsystemInterface.AddMappingContext` _returnvalue "/Game/Blueprints/Core/Input/IMC_Default.IMC_Default" 0 (struct))
      (`self.CastReference`
        (:`Return`
          (set `PlayerController.bShowMouseCursor` true (`self.ControllerRef`)))))))

(event `EnhancedInput|/Game/Blueprints/Core/Input/Actions/IA_MoveCamera`
  (params (ActionValue :type "Vector2D Structure") (ElapsedSeconds :type "Float (double-precision)") (TriggeredSeconds :type "Float (double-precision)") (InputAction :type "InputAction Object Reference" :default "/Game/Blueprints/Core/Input/Actions/IA_MoveCamera.IA_MoveCamera"))
  (bind (_returnvalue_roll _returnvalue_pitch _returnvalue_yaw) (`KismetMathLibrary.BreakRotator` (`self.GetControlRotation`)))
  (bind (_returnvalue_roll_2 _returnvalue_pitch_2 _returnvalue_yaw_2) (`KismetMathLibrary.BreakRotator` (`self.GetControlRotation`)))
  (:`Triggered`
    (`self.AddMovementInput` (`KismetMathLibrary.GetRightVector` (`KismetMathLibrary.MakeRotator` _returnvalue_roll_2 0.0 _returnvalue_yaw_2)) ActionValue_X)
    (`self.AddMovementInput` (`KismetMathLibrary.GetForwardVector` (`KismetMathLibrary.MakeRotator` 0.0 0.0 _returnvalue_yaw)) ActionValue_Y)))

(fn `MovementSpeedCalculation`
  (returns (MoveSensitivity :type "Float (double-precision)"))
  (return (`KismetMathLibrary.FClamp` (/ (`SpringArmComponent.TargetArmLength` (`self.SpringArm`)) 100.0) 5.0 20.0)))

(fn `UserConstructionScript`)