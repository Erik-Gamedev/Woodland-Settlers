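; BP_UnitComponent is a component in the Worker folder that makes its owning actor selectable by click.
; On BeginPlay it binds to the owner's OnClicked event.
; A click casts the first player controller to BP_CameraController, adds the owner to that controller's selection list, and prints a debug message.
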(event `self.ReceiveBeginPlay`
  (add `Actor.OnClicked` (`self.GetOwner`) (`|CreateDelegate` :!event `OnOwnerClicked`)))

(event `OnOwnerClicked`
  (params (TouchedActor :type "Actor Object Reference") (ButtonPressed :type "Key Structure" :default "None"))
  (`self.AddUnitToSelectionList`)
  (`KismetSystemLibrary.PrintString` "Selected"))

(event `AddUnitToSelectionList`
  (bind _asbp_camera_controller (cast `/Game/Blueprints/Camera/BP_CameraController` (`GameplayStatics.GetPlayerController` 0)))
  (`/Game/Blueprints/Camera/BP_CameraController.AddActorSelectedToList` _asbp_camera_controller (`self.GetOwner`)))